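; Final corridor trigger actor that starts the victory sequence when the main character overlaps its box.
; On overlap it disables the player controller's input and calls Victory on the character.
; After a short delay it turns on every LastRoomLights actor, then plays one light switch sound at the last light's location.
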(event `self.Box.OnComponentBeginOverlap`
  (params (OverlappedComponent :type "PrimitiveComponent Object Reference") (OtherActor :type "Actor Object Reference") (OtherComp :type "PrimitiveComponent Object Reference") (OtherBodyIndex :type Integer) (bFromSweep :type Boolean) (SweepResult :type "HitResult Structure (by ref)"))
  (bind _returnvalue (`GameplayStatics.GetPlayerController` 0))
  ;[0.7969 0.3237 0.3237] Final corridor colision event
  (bind _asmain_character (cast `/Game/Blueprints/MainCharacter` OtherActor))
  (`self.DisableInput` (cast `/Game/Blueprints/MainPlayerController` _returnvalue :!pure true) _returnvalue)
  (`/Game/Blueprints/MainCharacter.Victory` _asmain_character)
  (`KismetSystemLibrary.Delay` 3.5)
  (bind _outactors (`GameplayStatics.GetAllActorsOfClass` "/Game/Blueprints/LastRoomLights.LastRoomLights_C"))
  (for _array_element _outactors
    (`/Game/Blueprints/LastRoomLights.LightsOn` _array_element))
  (`GameplayStatics.PlaySoundAtLocation` "/Game/Audio/LightSwitcher.LightSwitcher" (`self.K2_GetActorLocation` _array_element) (struct) 0.6 1.0 0.0 null null null))

(fn `UserConstructionScript`)