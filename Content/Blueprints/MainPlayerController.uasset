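; Player controller that handles camera-relative character movement, pausing, input toggling and the player being caught.
; Movement scales Speed per axis, but each diagonal check tests its own axis twice, so any nonzero input gets the diagonal speed.
; PauseGame switches input mode, cursor and UI overlay; CaughtEvent runs once, disabling input, turning the camera to the enemy, then notifying the UI and playing sound.
; BeginPlay only prints a message for the GameInstance difficulty.
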(event `self.ReceiveBeginPlay`
  ;[1 0.04314 0.04314] Sets the difficulty of the game at the startup
  (switch `int` (`/Game/Blueprints/MainGameInstance.Difficulty` (cast `/Game/Blueprints/MainGameInstance` (`GameplayStatics.GetGameInstance`) :!pure true))
    (:`0`
      (`KismetSystemLibrary.PrintString` "to facil"))
    (:`1`
      (`KismetSystemLibrary.PrintString` "ta duro"))))

(event `InputAxis|MoveForward`
  (params (AxisValue :type "Float (single-precision)"))
  (bind _asmain_character (cast `/Game/Blueprints/MainCharacter` (`GameplayStatics.GetPlayerCharacter` 0) :!pure true))
  (bind _asmain_character_2 (cast `/Game/Blueprints/MainCharacter` (`GameplayStatics.GetPlayerCharacter` 0) :!pure true))
  ;[0.4 1 0.4] Character movement
  ;;[0.1 1 0.1] Move diagonal-forward speed
  (if (and (!= AxisValue 0.0) (!= (stale `InputAxis|MoveRight` AxisValue) 0.0))
    (`Pawn.AddMovementInput` _asmain_character (`SceneComponent.GetForwardVector` (`/Game/Blueprints/MainCharacter.Camera1` _asmain_character)) (* AxisValue (/ (`self.Speed`) 1.4)) false)
    (else
      ;;[0.1 1 0.1] Move forward speed
      (`Pawn.AddMovementInput` _asmain_character_2 (`SceneComponent.GetForwardVector` (`/Game/Blueprints/MainCharacter.Camera1` _asmain_character_2)) (* AxisValue (`self.Speed`)) false))))

(event `InputAxis|MoveRight`
  (params (AxisValue :type "Float (single-precision)"))
  (bind _asmain_character (cast `/Game/Blueprints/MainCharacter` (`GameplayStatics.GetPlayerCharacter` 0) :!pure true))
  (bind _asmain_character_2 (cast `/Game/Blueprints/MainCharacter` (`GameplayStatics.GetPlayerCharacter` 0) :!pure true))
  ;[0.4 1 0.4] Character movement
  (if (and (!= (stale `InputAxis|MoveForward` AxisValue) 0.0) (!= AxisValue 0.0))
    ;;[0.1 1 0.1] Move diagonal-right speed
    (`Pawn.AddMovementInput` _asmain_character_2 (`SceneComponent.GetRightVector` (`/Game/Blueprints/MainCharacter.Camera1` _asmain_character_2)) (* AxisValue (/ (`self.Speed`) 2.4)) false)
    (else
      ;;[0.1 1 0.1] Move right speed
      (`Pawn.AddMovementInput` _asmain_character (`SceneComponent.GetRightVector` (`/Game/Blueprints/MainCharacter.Camera1` _asmain_character)) (* AxisValue (* (`self.Speed`) 0.55)) false))))

(event `InputAction|Pause`
  (params (Key :type "Key Structure"))
  ;[0 1 1] Pause
  (:`Pressed`
    (`self.PauseGame` true)))

(event `PauseGame`
  (params (`paused?` :type Boolean))
  (bind _returnvalue (`GameplayStatics.GetPlayerController` 0))
  ;[0.733 0.1051 1] Pause event
  (bind _foundwidgets (`WidgetBlueprintLibrary.GetAllWidgetsOfClass` "/Game/Blueprints/Widgets/UI.UI_C"))
  (if `paused?`
    (bind _output (`|GetArrayItem` _foundwidgets))
    (`WidgetBlueprintLibrary.SetInputMode_UIOnlyEx` _returnvalue _output)
    (else
      (`WidgetBlueprintLibrary.SetInputMode_GameAndUIEx` _returnvalue _output)))
  (bind _output_get (set `self.bShowMouseCursor` `paused?`))
  (bind _returnvalue_2 (`GameplayStatics.SetGamePaused` _output_get))
  (`/Game/Blueprints/Widgets/UI.ShowBlackScreen` _output _returnvalue_2)
  (`/Game/Blueprints/Widgets/UI.ShowButtons` _output _returnvalue_2))

(event `CaughtEvent`
  (bind _asmain_character (cast `/Game/Blueprints/MainCharacter` (`GameplayStatics.GetPlayerCharacter` 0) :!pure true))
  ;[0.04314 0 0] Caught event
  (`/Engine/EditorBlueprintResources/StandardMacros.DoOnce` false
    (:`Completed`
      (`self.DisableInput` (`GameplayStatics.GetPlayerController` 0))
      (`/Engine/EditorBlueprintResources/StandardMacros.IsValid` (`/Game/Blueprints/MainCharacter.Enemy` _asmain_character)
        (:`Is Valid`
          (`/Game/Blueprints/MainCharacter.CameraToEnemy` _asmain_character))
        (:`Is Not Valid`
          _))
      (`KismetSystemLibrary.Delay` 1.0)
      (bind _foundwidgets (`WidgetBlueprintLibrary.GetAllWidgetsOfClass` "/Game/Blueprints/Widgets/UI.UI_C"))
      (`/Game/Blueprints/Widgets/UI.GetCaughtEvent` (`|GetArrayItem` _foundwidgets))
      (`GameplayStatics.PlaySound2D` null 1.0 1.0 0.0 null null))))

(event `SetInput`
  (params (`Enable?` :type Boolean))
  (bind _returnvalue (`GameplayStatics.GetPlayerController` 0))
  (if `Enable?`
    (`self.EnableInput` _returnvalue)
    (else
      (`self.DisableInput` _returnvalue))))

(fn `UserConstructionScript`)