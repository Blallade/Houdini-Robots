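; MusicManager is a Blueprint that controls the game's background music for the main theme and the ukulele main menu theme.
; Each play event takes a Play flag, either spawning a 2D sound, storing it and fading it in, or fading the stored one out.
; PlayVictoryMusic and PauseMainTheme are empty stubs, with the attempted pause and volume logic left disconnected.
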(event `PlayVictoryMusic`
  (params (`Play?` :type Boolean)))

(event `PlayMainTheme`
  (params (`Play?` :type Boolean))
  ;[0.549 0.1765 1] Play main theme
  (if `Play?`
    (bind _returnvalue (`GameplayStatics.SpawnSound2D` "/Game/Audio/Themes/OST_Houdini_Robots.OST_Houdini_Robots" 0.1 1.0 0.0 null false false))
    (bind _output_get (set `self.MainTheme` _returnvalue))
    (`AudioComponent.FadeIn` _returnvalue 0.5 1.0 0.0 "Linear")
    (`AudioComponent.FadeIn` _output_get 0.5 1.0 0.0 "Linear")
    (else
      (`AudioComponent.FadeOut` (`self.MainTheme`) 0.5 0.0 "Linear"))))

(event `PlayMainMenuTheme`
  (params (`Play?` :type Boolean))
  ;[0.549 0.1765 1] Play ukelele's theme
  (if `Play?`
    (bind _returnvalue (`GameplayStatics.SpawnSound2D` "/Game/Audio/Themes/OST_Houdini_Robots_main_menu.OST_Houdini_Robots_main_menu" 0.1 1.0 0.0 null false false))
    (bind _output_get (set `self.MainMenuTheme` _returnvalue))
    (`AudioComponent.FadeIn` _returnvalue 0.5 1.0 0.0 "Linear")
    (`AudioComponent.FadeIn` _output_get 0.5 1.0 0.0 "Linear")
    (else
      (`AudioComponent.FadeOut` (`self.MainMenuTheme`) 3.0 0.0 "Linear"))))

(event `PauseMainTheme`
  (params (`Pause?` :type Boolean))
  ;[1 0.1914 0.3927] Pause main theme (tried)
)

(fn `UserConstructionScript`)