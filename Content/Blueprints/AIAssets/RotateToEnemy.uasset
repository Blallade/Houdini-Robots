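; Behavior tree task that turns a StaticEnemy to face the main character.
; On tick it gets the controlled pawn from StaticEnemyController and reads its Enemy reference as the MainCharacter.
; It lerps the pawn's rotation along the shortest path toward a look-at rotation, scaled by delta time, then finishes successfully.
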(event `self.ReceiveTick`
  (params (OwnerActor :type "Actor Object Reference") (DeltaSeconds :type "Float (single-precision)"))
  ;[1 0.5836 0.1458] Task that rotates the enemy to the main character
  (bind _asstatic_enemy_controller (cast `/Game/Blueprints/AIAssets/StaticEnemyController` OwnerActor))
  (bind _asstatic_enemy (cast `/Game/Blueprints/StaticEnemy` (`Controller.K2_GetPawn` _asstatic_enemy_controller)))
  (bind _asmain_character (cast `/Game/Blueprints/MainCharacter` (`/Game/Blueprints/StaticEnemy.enemy` _asstatic_enemy)))
  (`Actor.K2_SetActorRotation` _asstatic_enemy (`KismetMathLibrary.RLerp` (`Actor.K2_GetActorRotation` _asstatic_enemy) (`KismetMathLibrary.FindLookAtRotation` (`Actor.K2_GetActorLocation` _asstatic_enemy) (`Actor.K2_GetActorLocation` _asmain_character)) (* DeltaSeconds 10.0) true) false)
  (`self.FinishExecute` true))