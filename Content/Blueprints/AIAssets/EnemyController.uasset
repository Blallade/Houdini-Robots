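; AI controller for enemies that starts a behavior tree and supplies it with level target points.
; On BeginPlay it waits briefly, runs the tree, then gathers all TargetPoint actors in the level.
; It writes the first twelve into numbered blackboard keys, Point1 to Point12, by fixed array index with no count check, so point assignment follows the query's return order.
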(event `self.ReceiveBeginPlay`
  (bind _returnvalue (`AIBlueprintHelperLibrary.GetBlackboard` null))
  ;[0.4219 0.4219 0.4219] Begin play set up
  (`KismetSystemLibrary.Delay` 0.2)
  (`self.RunBehaviorTree` (`self.BehaviorTree`))
  (bind _outactors (`GameplayStatics.GetAllActorsOfClass` "/Script/Engine.TargetPoint"))
  (`BlackboardComponent.SetValueAsObject` _returnvalue "Point1" (`|GetArrayItem` _outactors))
  (`BlackboardComponent.SetValueAsObject` _returnvalue "Point2" (`|GetArrayItem` _outactors 1))
  (`BlackboardComponent.SetValueAsObject` _returnvalue "Point3" (`|GetArrayItem` _outactors 2))
  (`BlackboardComponent.SetValueAsObject` _returnvalue "Point4" (`|GetArrayItem` _outactors 3))
  (`BlackboardComponent.SetValueAsObject` _returnvalue "Point5" (`|GetArrayItem` _outactors 4))
  (`BlackboardComponent.SetValueAsObject` _returnvalue "Point6" (`|GetArrayItem` _outactors 5))
  (`BlackboardComponent.SetValueAsObject` _returnvalue "Point7" (`|GetArrayItem` _outactors 6))
  (`BlackboardComponent.SetValueAsObject` _returnvalue "Point8" (`|GetArrayItem` _outactors 7))
  (`BlackboardComponent.SetValueAsObject` _returnvalue "Point9" (`|GetArrayItem` _outactors 8))
  (`BlackboardComponent.SetValueAsObject` _returnvalue "Point10" (`|GetArrayItem` _outactors 9))
  (`BlackboardComponent.SetValueAsObject` _returnvalue "Point11" (`|GetArrayItem` _outactors 10))
  (`BlackboardComponent.SetValueAsObject` _returnvalue "Point12" (`|GetArrayItem` _outactors 11)))

(fn `UserConstructionScript`)